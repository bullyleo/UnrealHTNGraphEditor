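; BP_UseWeapon is a planner action for the Shooter2 sample that makes a BP_Agent use its weapon.
; On initialization it prints the operator parameter as a world-state name and caches the pawn as a BP_Agent.
; Execution calls UseWeapon on the agent and immediately finishes as successful.
; It reports actual effects as a world-state map built from the agent's current ammo and its enemy's health.
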(event EventInitializeAction
  (params (OwnerController :type AI%20Controller%20Object%20Reference) (ControlledPawn :type Pawn%20Object%20Reference) (OperatorParam :type Byte :default 0))
  (Development|PrintString 0 (Utilities|String|Append "Task : Use Weapon | Parameter : " (Utilities|String|EnumtoString (Utilities|Enum|ByteToEnumEShooter2_WorldState OperatorParam))))
  (Variables|Default|SetOwnerPawnRef (.AsBP%20Agent (Utilities|Casting|CastToBP_Agent ControlledPawn))))

(event EventReceiveExecuteAction
  (params (OwnerController :type AI%20Controller%20Object%20Reference) (ControlledPawn :type Pawn%20Object%20Reference) (OperatorParam :type Byte :default 0))
  (Default|UseWeapon (Variables|Default|GetOwnerPawnRef))
  (Class|HTNOperatorBlueprintBase|FinishExecute true))

(fn GetActualEffectsInternal
  (params (OwnerController :type AI%20Controller%20Object%20Reference) (ControlledPawn :type Pawn%20Object%20Reference))
  (return (Utilities|Map|MakeMap (Utilities|Enum|LiteralenumEShooter2_WorldState "NewEnumerator7") (Variables|/Game/Sample_Shooter2WithBlueprint/BP_Agent.BP_Agent_C|GetAmmo (Variables|Default|GetOwnerPawnRef)) (Utilities|Enum|LiteralenumEShooter2_WorldState "NewEnumerator0") (Default|GetEnemyHealth (Variables|Default|GetOwnerPawnRef)))))