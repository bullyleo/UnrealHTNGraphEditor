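; Sample shooter AI agent Blueprint driven by a Hierarchical Task Network (HTN) planner.
; On BeginPlay it builds the HTN_Shooter2 domain, generates a plan and runs operators on a looping timer, replanning when all tasks finish.
; Helper functions supply world data: random patrol point, weapon spawn location, enemy health and a destination chosen by world-state key.
; UseWeapon damages the enemy and spends ammo, while PickupAmmo only prints a message.
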(event OnAllTaskFinished(HTN)
  (bind _htn (Variables|Default|GetHTN))
  (Class|HTNComponent|BuildHTNDomain _htn "/Game/Sample_Shooter2/HTN_Shooter2.HTN_Shooter2")
  (Class|HTNComponent|GeneratePlan _htn))

(event Custom|UseWeapon
  (bind _ammo (Variables|Default|GetAmmo))
  (Development|PrintString "beeow beeow")
  (Game|Damage|ApplyDamage (Variables|Default|GetEnemyRef) 1.0 0 0)
  (if (> _ammo 0)
    (Math|Integer|DecrementInt _ammo)))

(event Custom|PickupAmmo
  (Development|PrintString "PickupAmmo"))

(event Custom|ExecuteOperators
  (Class|HTNComponent|ExecuteOperators (Variables|Default|GetHTN)))

(event EventBeginPlay
  (bind _htn (Variables|Default|GetHTN))
  (Class|HTNComponent|BuildHTNDomain _htn "/Game/Sample_Shooter2/HTN_Shooter2.HTN_Shooter2")
  (Class|HTNComponent|GeneratePlan _htn)
  (Utilities|Time|SetTimerbyEvent (delegate Custom|ExecuteOperators) 0.1 true))

(fn ConstructionScript)

(fn GetRandomLocation
  (bind _output_get (Variables|Default|SetPatrolLocation (.RandomLocation (AI|Navigation|GetRandomReachablePointinRadius (Math|Vector|MakeVector 0.0 0.0 0.0) 5e+02 0 0))))
  (Rendering|Debug|DrawDebugSphere _output_get 5e+01 12 "(R=1.000000,G=0.000000,B=0.000000,A=1.000000)" 2.0 1e+01))

(fn GetDestination
  (params (OperatorParam :type Byte))
  (switch Utilities|FlowControl|Switch|SwitchonEShooter2_WorldState (Utilities|Enum|ByteToEnumEShooter2_WorldState OperatorParam)
    (:NewEnumerator1
      (return (Transformation|GetActorLocation (Variables|Default|GetEnemyRef))))
    (:NewEnumerator3
      (return (Variables|Default|GetPatrolLocation)))
    (:NewEnumerator4
      (return (Variables|Default|GetWeaponLocation)))))

(fn GetWeaponLocation
  (Variables|Default|SetWeaponLocation (Transformation|GetActorLocation (Variables|Default|GetWeaponSpawnLocation))))

(fn GetEnemyHealth
  (bind _enemyref (Variables|Default|GetEnemyRef))
  (Utilities|IsValid _enemyref
    (:Is%20Valid
      (return (Variables|/Game/Sample_Shooter2WithBlueprint/BP_Enemy.BP_Enemy_C|GetHealth _enemyref)))
    (:Is%20Not%20Valid
      (return 0))))