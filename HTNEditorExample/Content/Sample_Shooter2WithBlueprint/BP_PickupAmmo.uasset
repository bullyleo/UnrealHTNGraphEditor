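; Planner task for the Shooter2 Blueprint sample that makes an agent pick up ammo.
; On initialization it prints the task name with its world-state parameter and caches the controlled pawn as BP_Agent.
; Execution calls PickupAmmo on that agent and immediately finishes as successful.
; It reports its effect as a map setting one world-state key to 1, meaning true.
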(event EventInitializeAction
  (params (OwnerController :type AI%20Controller%20Object%20Reference) (ControlledPawn :type Pawn%20Object%20Reference) (OperatorParam :type Byte :default 0))
  (Development|PrintString 0 (Utilities|String|Append "Task : Pickup Ammo | Parameter : " (Utilities|String|EnumtoString (Utilities|Enum|ByteToEnumEShooter2_WorldState OperatorParam))))
  (Variables|Default|SetOwnerPawnRef (.AsBP%20Agent (Utilities|Casting|CastToBP_Agent ControlledPawn))))

(event EventReceiveExecuteAction
  (params (OwnerController :type AI%20Controller%20Object%20Reference) (ControlledPawn :type Pawn%20Object%20Reference) (OperatorParam :type Byte :default 0))
  (Default|PickupAmmo (Variables|Default|GetOwnerPawnRef))
  (Class|HTNOperatorBlueprintBase|FinishExecute true))

(fn GetActualEffectsInternal
  (params (OwnerController :type AI%20Controller%20Object%20Reference) (ControlledPawn :type Pawn%20Object%20Reference))
  (return (Utilities|Map|MakeMap (Utilities|Enum|LiteralenumEShooter2_WorldState "NewEnumerator2") (Class|KismetSystemLibrary|MakeLiteralInteger 1))))