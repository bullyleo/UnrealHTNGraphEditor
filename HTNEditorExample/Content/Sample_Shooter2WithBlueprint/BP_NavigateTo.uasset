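; Navigate To planner action for the Shooter2 sample that moves a BP_Agent to a destination chosen by its operator parameter.
; Execution asks the agent for the location and runs AI MoveTo behind a DoOnce, reporting success or failure and then resetting.
; Its reported world-state effects depend on the parameter, covering current location, enemy visibility or weapon possession.
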(event Custom|ResetDoOnce
  (Utilities|FlowControl|DoOnce false) ; enters at Reset
)

(event EventInitializeAction
  (params (OwnerController :type AI%20Controller%20Object%20Reference) (ControlledPawn :type Pawn%20Object%20Reference) (OperatorParam :type Byte :default 0))
  (Variables|Default|SetOperatorParam OperatorParam)
  (Development|PrintString 0 (Utilities|String|Append "Task : Navigate To | Parameter : " (Utilities|String|EnumtoString (Utilities|Enum|ByteToEnumEShooter2_WorldState OperatorParam))))
  (Variables|Default|SetOwnerPawnRef (.AsBP%20Agent (Utilities|Casting|CastToBP_Agent ControlledPawn))))

(event EventReceiveExecuteAction
  (params (OwnerController :type AI%20Controller%20Object%20Reference) (ControlledPawn :type Pawn%20Object%20Reference) (OperatorParam :type Byte :default 0))
  (Utilities|FlowControl|DoOnce false
    (:Completed
      (AI|AIMoveTo OwnerController (Default|GetDestination (Variables|Default|GetOwnerPawnRef) OperatorParam) 0 1e+02 "Default" "Default" true true
        (:OnRequestFailed
          (Class|HTNOperatorBlueprintBase|FinishExecute false))
        (:OnMoveFinished
          (Class|HTNOperatorBlueprintBase|FinishExecute true)))
      (CallFunction|ResetDoOnce))))

(fn GetActualEffectsInternal
  (params (OwnerController :type AI%20Controller%20Object%20Reference) (ControlledPawn :type Pawn%20Object%20Reference))
  (switch Utilities|FlowControl|Switch|SwitchonEShooter2_WorldState (Utilities|Enum|ByteToEnumEShooter2_WorldState (Variables|Default|GetOperatorParam))
    (:NewEnumerator1
      ;[1 1 1] Operator Param : Enemy Actor
      (return (Utilities|Map|MakeMap (Utilities|Enum|LiteralenumEShooter2_WorldState "NewEnumerator5") (Math|Conversions|ToInteger(Byte) (Utilities|Enum|LiteralenumEShooter2_WorldState "NewEnumerator3")) (Utilities|Enum|LiteralenumEShooter2_WorldState "NewEnumerator6") (Class|KismetSystemLibrary|MakeLiteralInteger 1))))
    (:NewEnumerator3
      ;[1 1 1] Operator Param : Move Destination
      (return (Utilities|Map|MakeMap (Utilities|Enum|LiteralenumEShooter2_WorldState "NewEnumerator5") (Math|Conversions|ToInteger(Byte) (Utilities|Enum|LiteralenumEShooter2_WorldState "NewEnumerator3")))))
    (:NewEnumerator4
      ;[1 1 1] Operator Param : Pickup Location
      (return (Utilities|Map|MakeMap (Utilities|Enum|LiteralenumEShooter2_WorldState "NewEnumerator2") (Class|KismetSystemLibrary|MakeLiteralInteger 1))))))